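; Recognizer actor that moves its Car component along the spline of a referenced SplineBP in a continuous loop.
; Each tick it advances a distance by Speed times delta time, resetting to zero once it reaches the spline's length.
; The car's world location and rotation are then set from the spline at that distance, without sweeping.
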(event EventBeginPlay)

(event Collision|EventActorBeginOverlap
  (params (OtherActor :type Actor%20Object%20Reference)))

(event EventTick
  (params (DeltaSeconds :type Float%20%28single-precision%29))
  (bind _car (Variables|Default|Getcar))
  (bind _spline_bp (Variables|Default|GetSpline_BP))
  (bind _spline (Variables|/Game/Blueprints/Spline_BP.Spline_BP_C|GetSpline _spline_bp))
  (if (> (Spline|GetSplineLength _spline) (Variables|Default|GetDistancealongspline))
    (Variables|Default|SetDistancealongspline (+ (* DeltaSeconds (Variables|Default|Getspeed)) (Variables|Default|GetDistancealongspline)))
    (else
      (Variables|Default|SetDistancealongspline 0.0)))
  (Transformation|SetWorldLocation _car (Spline|GetLocationatDistanceAlongSpline _spline (Variables|Default|GetDistancealongspline) "World") false false)
  (Transformation|SetWorldRotation _car (Spline|GetRotationatDistanceAlongSpline _spline (Variables|Default|GetDistancealongspline) "World") false false))

(fn ConstructionScript)