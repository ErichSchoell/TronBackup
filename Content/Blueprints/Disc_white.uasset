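; Disc_white is a networked VR disc projectile that flies out, then homes back to its homing target, by default player 0's right controller.
; EnableMovement switches it from physics to projectile movement.
; On the server, Tick enables homing once velocity turns back against the player-to-enemy direction and destroys the disc near the target.
; Hits spawn shield or regular impact effects, and the server breaks HexWall pieces.
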(event Custom|Enable%20Movement
  (params (Local%20Velocity :type Vector))
  (bind _projectilemovement (Variables|Default|GetProjectileMovement))
  (Game|Components|ProjectileMovement|SetVelocityinLocalSpace _projectilemovement Local%20Velocity)
  (Physics|SetSimulatePhysics (Variables|Default|GetDisc) false)
  (Components|Activation|Activate _projectilemovement false))

(event Custom|Enable%20Homing
  (bind _projectilemovement (Variables|Default|GetProjectileMovement))
  (Variables|/Script/Engine.ProjectileMovementComponent|SetHomingTargetComponent _projectilemovement (Variables|Default|GetHomingTarget))
  (Variables|/Script/Engine.ProjectileMovementComponent|SetbIsHomingProjectile _projectilemovement true))

(event EventBeginPlay
  (bind _asvr_game_mode (Utilities|Casting|CastToVR_GameMode (Game|GetGameMode)))
  (Variables|Default|SetVR_GameMode _asvr_game_mode)
  (CallFunction|InitDisc))

(event EventTick
  (params (DeltaSeconds :type Float%20%28single-precision%29))
  (Networking|SwitchHasAuthority
    (:Authority
      (if (Components|Activation|IsActive (Variables|Default|GetProjectileMovement))
        (Utilities|IsValid (Variables|Default|GetHomingTarget)
          (:Is%20Valid
            (Utilities|FlowControl|Sequence
              (:then_0
                ;[1 1 1] Enable Homing when Disc is returning
                (if (> (Class|KismetMathLibrary|DegAcos (Math|Vector|DotProduct (Variables|Default|GetDirectionFromPlayerToEnemy) (Math|Vector|Normalize (* (Transformation|GetVelocity) "1.000000,1.000000, 0")))) 9e+01)
                  (Utilities|FlowControl|DoOnce true :!label _label
                    (:Completed
                      (CallFunction|EnableHoming)))
                  (else
                    (goto _label Reset))))
              (:then_1
                ;[1 1 1] Destroy Disc when returned
                (if (and (Variables|/Script/Engine.ProjectileMovementComponent|GetbIsHomingProjectile (Variables|Default|GetProjectileMovement)) (< (Math|Vector|VectorLength (- (Transformation|GetActorLocation) (Transformation|GetWorldLocation (Variables|Default|GetHomingTarget)))) 1e+02))
                  (Actor|DestroyActor))))))))))

(event Collision|EventHit
  (params (MyComp :type Primitive%20Component%20Object%20Reference) (Other :type Actor%20Object%20Reference) (OtherComp :type Primitive%20Component%20Object%20Reference) (bSelfMoved :type Boolean) (HitLocation :type Vector) (HitNormal :type Vector) (NormalImpulse :type Vector :default "0, 0, 0") (Hit :type Hit%20Result%20Structure%20%28by%20ref%29))
  (Effects|SpawnEmitteratLocation (select (Components|ComponentHasTag OtherComp "Shield") "/Game/ParticleEffects/Shield_Collision.Shield_Collision" "/Game/ParticleEffects/Collision.Collision") HitLocation (Math|Rotator|FindLookatRotation HitLocation (+ HitLocation HitNormal)))
  (Networking|SwitchHasAuthority
    (:Authority
      (CallFunction|HitHexWall Other OtherComp HitLocation))))

(fn ConstructionScript)

(fn HitHexWall
  (params (Other%20Actor :type Actor%20Object%20Reference) (Component :type Primitive%20Component%20Object%20Reference) (Location :type Vector))
  (bind _ashex_wall (Utilities|Casting|CastToHexWall Other%20Actor)
    (:then
      (Default|DestroyHexPiece _ashex_wall Component Location))
    (:CastFailed
      _))
  (return))

(fn InitDisc
  (Class|ActorComponent|SetIsReplicated (Variables|Default|GetProjectileMovement) true)
  (Utilities|IsValid (Variables|Default|GetHomingTarget)
    (:Is%20Valid
      (Variables|Default|SetDirectionFromPlayerToEnemy (Class|KismetMathLibrary|GetDirectionVector (* (Transformation|GetWorldLocation (Variables|Default|GetHomingTarget)) "0.000000,1.000000, 0") (Math|Vector|MakeVector 0.0 0.0 0.0)) :!label _label))
    (:Is%20Not%20Valid
      (bind _asvr_character (Utilities|Casting|CastToVR_Character (Game|Player|GetPlayerPawn 0))
        (:then
          (Variables|Default|SetHomingTarget (Variables|/Game/Blueprints/VR_Character.VR_Character_C|Getvr_controller_R _asvr_character))
          (goto _label))
        (:CastFailed
          _))))
  (return))