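; Game state for a two-player networked VR match that decides the winner from each player's hex wall count.
; Every tick it checks for a wall count reaching zero, or compares counts when time runs out.
; Wins fire once, using authority (host as player one) to pick which tagged win/lose text and sound each machine gets.
; A Matinee then plays and the server reloads the level, after a delay for wins but immediately on draws.
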(event Custom|WinPlayer2
  (Networking|SwitchHasAuthority
    (:Authority
      (CallFunction|UnhideWinLoseText false "NewEnumerator0")
      (Audio|SpawnSound2D "/Game/Sound/Goal_Against_Hit_sfx_Cue.Goal_Against_Hit_sfx_Cue"))
    (:Remote
      (CallFunction|UnhideWinLoseText true "NewEnumerator1")
      (Audio|SpawnSound2D "/Game/Sound/Goal_Hit_sfx_Cue.Goal_Hit_sfx_Cue"))))

(event Custom|WinPlayer1
  (Networking|SwitchHasAuthority
    (:Authority
      (CallFunction|UnhideWinLoseText true "NewEnumerator0")
      (Audio|SpawnSound2D "/Game/Sound/Goal_Hit_sfx_Cue.Goal_Hit_sfx_Cue"))
    (:Remote
      (CallFunction|UnhideWinLoseText false "NewEnumerator1")
      (Audio|SpawnSound2D "/Game/Sound/Goal_Against_Hit_sfx_Cue.Goal_Against_Hit_sfx_Cue"))))

(event EventBeginPlay
  (bind _outactors (Actor|GetAllActorsOfClass "/Game/Blueprints/YouWinBP.YouWinBP_C"))
  (Variables|Default|SetWinRefs _outactors)
  (bind _outactors_2 (Actor|GetAllActorsOfClass "/Game/Blueprints/YouLoseBP.YouLoseBP_C"))
  (Variables|Default|SetLoseRefs _outactors_2))

(event EventTick
  (params (DeltaSeconds :type Float%20%28single-precision%29))
  (Utilities|CheckWinConditions
    (:P1%20Win
      (Utilities|FlowControl|DoOnce false
        (:Completed
          (CallFunction|WinPlayer1)
          (Utilities|FlowControl|Delay 3.0 :!label _label))))
    (:Draw
      _)
    (:P2%20Win
      (Utilities|FlowControl|DoOnce false
        (:Completed
          (CallFunction|WinPlayer2)
          (goto _label)))))
  (bind _outactors (Actor|GetAllActorsOfClass "/Script/Engine.MatineeActor"))
  (Audio|Components|Audio|Play (Utilities|Array|Get(acopy) _outactors 1))
  (Networking|SwitchHasAuthority
    (:Authority
      (bind _returnvalue (Game|GetCurrentLevelName true))
      (Development|ExecuteConsoleCommand (Utilities|String|Append "ServerTravel " _returnvalue "?listen")))))

(fn ConstructionScript)

(fn UnhideWinLoseText
  (params (Win :type Boolean) (Player :type MyTags%20Enum))
  (if Win
    (bind _array_element (Utilities|Array|ForEachLoopwithBreak (Variables|Default|GetWinRefs) :!label _label)
      (:LoopBody
        (if (Utilities|Enum|Equal(Enum) (Variables|/Game/Blueprints/YouWinBP.YouWinBP_C|GetPlayerTag _array_element) Player)
          (Rendering|SetActorHiddenInGame _array_element false)
          (goto _label Break)))
      (:Completed
        (return)))
    (else
      (bind _array_element_2 (Utilities|Array|ForEachLoopwithBreak (Variables|Default|GetLoseRefs) :!label _label_2)
        (:LoopBody
          (if (Utilities|Enum|Equal(Enum) (Variables|/Game/Blueprints/YouLoseBP.YouLoseBP_C|GetPlayerTag _array_element_2) Player)
            (Rendering|SetActorHiddenInGame _array_element_2 false)
            (goto _label_2 Break)))
        (:Completed
          (return))))))