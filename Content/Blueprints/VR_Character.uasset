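; Networked VR player character for a two-player disc game, with a thrown disc in the right hand and a shield in the left.
; Physics handles carry both items; the authority spawns discs, and trigger release launches them at boosted hand velocity.
; The left trigger scales the shield through a timeline.
; Hand and head transforms replicate via the server, PlayerTag sets player colours, and mouse look covers play without an HMD.
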(event Custom|Spawn%20Disc
  (bind _discspawnpoint (Variables|Default|GetDiscSpawnPoint))
  (Effects|SpawnEmitterAttached "/Game/ParticleEffects/Disk_Catch.Disk_Catch" (Variables|Default|GetDiscSpawnPoint) "None" "0, 0, 0" "0, 0, 0" "SnapToTarget")
  (Utilities|FlowControl|Delay 0.1)
  (bind _returnvalue (Game|SpawnActorfromClass "/Game/Blueprints/Disc.Disc_C" (Math|Transform|MakeTransform (+ (Transformation|GetWorldLocation _discspawnpoint) (* (Math|Vector|GetForwardVector _discspawnpoint) 1e+01)) (Transformation|GetWorldRotation _discspawnpoint) "1.000000,1.000000,1.000000") "AlwaysSpawn" 0 self (Variables|Default|Getvr_controller_R)))
  (Variables|Default|SetSpawnedDisc _returnvalue)
  (CallFunction|GrabDisc))

(event Custom|Server_UpdateTrackedTransforms
  (params (LeftHandTransform :type Transform) (RightHandTransform :type Transform) (HeadTransform :type Transform%20%28by%20ref%29))
  (Variables|Default|SetLeftHandTransform LeftHandTransform)
  (Variables|Default|SetRightHandTransform RightHandTransform)
  (Transformation|SetRelativeTransform (Variables|MyCharacter|GetFirstPersonCamera) HeadTransform false false))

(event Custom|Deactivate%20Shield
  (Collision|SetCollisionEnabled (Variables|Default|GetShield) "PhysicsOnly")
  (bind _scale (Timeline|ShieldScaling Reverse)
    (:Update
      (Variables|Default|SetShieldScale _scale))))

(event Custom|Grab%20Disc
  (bind _spawneddisc (Variables|Default|GetSpawnedDisc))
  (Class|PhysicsHandleComponent|GrabComponent (Variables|Default|GetPhysicsHandleR) (Variables|/Game/Blueprints/Disc.Disc_C|GetDisc _spawneddisc) "None" (Transformation|GetActorLocation _spawneddisc) true))

(event Custom|Activate%20Shield
  (Collision|SetCollisionEnabled (Variables|Default|GetShield) "QueryAndPhysics")
  (bind _scale (Timeline|ShieldScaling Play)
    (:Update
      (Variables|Default|SetShieldScale _scale))))

(event Custom|Release%20Disc
  (bind _spawneddisc (Variables|Default|GetSpawnedDisc))
  (bind _returnvalue (Transformation|GetVelocity _spawneddisc))
  (bind _returnvalue_2 (Transformation|GetActorTransform _spawneddisc))
  (bind _returnvalue_3 (Math|Transform|InverseTransformDirection _returnvalue_2 _returnvalue))
  (Utilities|IsValid _spawneddisc
    (:Is%20Valid
      (if (not (Components|Activation|IsActive (Variables|/Game/Blueprints/Disc.Disc_C|GetProjectileMovement _spawneddisc)))
        (Physics|Components|PhysicsHandle|ReleaseComponent (Variables|Default|GetPhysicsHandleR))
        (Default|EnableMovement _spawneddisc (* (Math|Vector|Normalize _returnvalue_3) (+ (* (Math|Vector|VectorLength _returnvalue_3) 1.8) 2e+02)))))))

(event EventTick
  (params (DeltaSeconds :type Float%20%28single-precision%29))
  (bind _returnvalue (Utilities|Time|GetWorldDeltaSeconds))
  (bind _mesh (Variables|Character|GetMesh))
  (bind _firstpersoncamera (Variables|MyCharacter|GetFirstPersonCamera))
  (bind _returnvalue_2 (Transformation|GetRelativeTransform _mesh))
  (bind _returnvalue_3 (Transformation|GetRelativeTransform _firstpersoncamera))
  (bind _returnvalue_4 (Class|KismetMathLibrary|TInterpto _returnvalue_2 _returnvalue_3 _returnvalue 1e+01))
  (Utilities|FlowControl|Sequence
    (:then_0
      (Networking|SwitchHasAuthority
        (:Authority
          (Utilities|IsValid (Variables|Default|GetSpawnedDisc)
            (:Is%20Valid
              (goto _label Reset))
            (:Is%20Not%20Valid
              (Utilities|FlowControl|DoOnce false :!label _label
                (:Completed
                  (CallFunction|SpawnDisc))))))))
    (:then_1
      (CallFunction|SetControllerTargets)
      (CallFunction|SetShieldScale)
      (|ShieldDebugLines)
      (Transformation|SetRelativeTransform _mesh (Math|Transform|MakeTransform (.location _returnvalue_4) (Math|Rotator|MakeRotator 0.0 0.0 (.yaw (.rotation _returnvalue_4))) (.scale _returnvalue_4)) false false))
    (:then_2
      (CallFunction|UpdateTransformsLocally)
      (CallFunction|ServerUpdateTrackedTransforms (Variables|Default|GetLeftHandTransform) (Variables|Default|GetRightHandTransform) (Transformation|GetRelativeTransform (Variables|MyCharacter|GetFirstPersonCamera))))))

(event EventBeginPlay
  (CallFunction|InitCharacter))

(event Input|AxisEvents|InputAxisTurn
  (params (AxisValue :type Float%20%28single-precision%29))
  ;[1 1 1] MouseControl if no HMD detected
  (Transformation|AddWorldRotation (Variables|MyCharacter|GetFirstPersonCamera) (Math|Rotator|MakeRotator 0.0 0.0 AxisValue) false false))

(event Input|AxisEvents|InputAxisLookUp
  (params (AxisValue :type Float%20%28single-precision%29))
  ;[1 1 1] MouseControl if no HMD detected
  (Transformation|AddLocalRotation (Variables|MyCharacter|GetFirstPersonCamera) (Math|Rotator|MakeRotator 0.0 (* AxisValue -1.0) 0.0) false false))

(event Input|KeyboardEvents|MotionControllerRightTrigger
  (params (Key :type Key%20Structure :default "AnyKey"))
  (:Released
    (CallFunction|ReleaseDisc)))

(event Input|KeyboardEvents|MotionControllerLeftTrigger
  (params (Key :type Key%20Structure :default "AnyKey"))
  (bind _vr_controller_l (Variables|Default|Getvr_controller_L))
  (:Pressed
    (CallFunction|ActivateShield)
    ;[1 1 1] Shield sound
    (Audio|SpawnSoundAttached "/Game/Sound/Shield_ToggleOn_sfx_Cue.Shield_ToggleOn_sfx_Cue" _vr_controller_l)
    (Components|Activation|ToggleActive (Variables|Default|GetShield_Active_Cue)))
  (:Released
    (CallFunction|DeactivateShield)
    (Components|Activation|ToggleActive (Variables|Default|GetShield_Active_Cue))
    (Audio|SpawnSoundAttached "/Game/Sound/Shield_ToggleOff_sfx_Cue.Shield_ToggleOff_sfx_Cue" _vr_controller_l)))

(event Input|KeyboardEvents|SpaceBar
  (params (Key :type Key%20Structure :default "AnyKey"))
  (:Pressed
    (Variables|Default|SetPlayer_Ready true)
    (Development|PrintString "Player_ready" false)))

(fn ConstructionScript)

(fn InitCharacter
  (bind _shield (Variables|Default|GetShield))
  (bind _firstpersoncamera (Variables|MyCharacter|GetFirstPersonCamera))
  (Class|PhysicsHandleComponent|GrabComponent (Variables|Default|GetPhysicsHandleL) _shield "None" (Transformation|GetWorldLocation (Variables|Default|GetShield)) true)
  (Collision|SetCollisionEnabled _shield "QueryAndPhysics")
  ;[1 1 1] Enable Mouse Control if no HMD connected
  (if (Class|HeadMountedDisplayFunctionLibrary|IsHeadMountedDisplayEnabled)
    _
    (else
      (Variables|/Script/Engine.CameraComponent|SetbLockToHmd _firstpersoncamera false)
      (Variables|/Script/Engine.CameraComponent|SetbUsePawnControlRotation _firstpersoncamera false)))
  (return))

(fn SetControllerTargets
  (bind _discspawnpoint (Variables|Default|GetDiscSpawnPoint))
  (Class|PhysicsHandleComponent|SetTargetLocationandRotation (Variables|Default|GetPhysicsHandleR) (Transformation|GetWorldLocation _discspawnpoint) (Transformation|GetWorldRotation _discspawnpoint))
  (Class|PhysicsHandleComponent|SetTargetLocationandRotation (Variables|Default|GetPhysicsHandleL) (Transformation|GetWorldLocation (Variables|Default|GetShieldSpawnPoint)) "0.000000,0.000000,90.000000")
  (return))

(fn SetShieldScale
  (if (!= (Math|Vector|VectorLength (Variables|/Script/Engine.SceneComponent|GetRelativeScale3D (Variables|Default|GetShield))) (Math|Vector|VectorLength (Variables|Default|GetShieldScale)))
    (Transformation|SetRelativeScale3D (Variables|Default|GetShield) (Variables|Default|GetShieldScale)))
  (return))

(fn DrawLine
  (params (From :type Scene%20Component%20Object%20Reference) (To :type Scene%20Component%20Object%20Reference) (LineColor :type Linear%20Color%20Structure) (Thickness :type Float%20%28single-precision%29))
  (Rendering|Debug|DrawDebugLine (Transformation|GetWorldLocation From) (Transformation|GetWorldLocation To) LineColor 0.0 Thickness))

(fn UpdateTransformsLocally
  (bind (_outposition _outorientation) (Class|SteamVRFunctionLibrary|GetHandPositionandOrientation 0 "Right"))
  (bind (_outposition_2 _outorientation_2) (Class|SteamVRFunctionLibrary|GetHandPositionandOrientation 0 "Left"))
  (if (Pawn|IsLocallyControlled)
    (Variables|Default|SetLeftHandTransform (Math|Transform|MakeTransform _outposition_2 _outorientation_2))
    (Variables|Default|SetRightHandTransform (Math|Transform|MakeTransform _outposition _outorientation))))

(fn OnRepLeftHandTransform
  (Transformation|SetRelativeTransform (Variables|Default|GetControllerL) (Variables|Default|GetLeftHandTransform) false false))

(fn OnRepRightHandTransform
  (Transformation|SetRelativeTransform (Variables|Default|GetControllerR) (Variables|Default|GetRightHandTransform) false false))

(fn OnRepPlayerTag
  (bind _spawneddisc (Variables|Default|GetSpawnedDisc))
  (Rendering|Material|SetMaterial (Variables|Default|Getvr_controller_L) 1 (Utilities|Select :Index (Variables|Default|GetPlayerTag) :NewEnumerator0 "/Game/Materials/basic_glow_red.basic_glow_red" :NewEnumerator1 "/Game/Materials/basic_glow_white3.basic_glow_white3"))
  (Rendering|Material|SetMaterial (Variables|Default|GetShield) 0 (Utilities|Select :Index (Variables|Default|GetPlayerTag) :NewEnumerator0 "/Game/Materials/shield_new_red.shield_new_red" :NewEnumerator1 "/Game/Materials/shield_new_white.shield_new_white"))
  (Utilities|IsValid _spawneddisc
    (:Is%20Valid
      (Default|InitDisc _spawneddisc))))