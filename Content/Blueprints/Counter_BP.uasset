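; Counter actor that shows a player's hit count through a row of wall pieces.
; HexWallToggleCall reveals the pieces one at a time, looping through a Delay of ActivationDelay, then resets the index.
; HitCounter, when the hit player matches PlayerTagSet, switches the current piece to that player's red or white "off" goal material and advances the shared index, which it never resets.
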(event EventBeginPlay)

(event Collision|EventActorBeginOverlap
  (params (OtherActor :type Actor%20Object%20Reference)))

(event EventTick
  (params (DeltaSeconds :type Float%20%28single-precision%29)))

(event EventHexWallToggleCall
  (bind _5 (Variables|Default|Get5))
  (bind _1 (Variables|Default|Get1))
  (bind _2 (Variables|Default|Get2))
  (bind _3 (Variables|Default|Get3))
  (bind _4 (Variables|Default|Get4))
  (bind _6 (Variables|Default|Get6))
  (bind _7 (Variables|Default|Get7))
  (bind _8 (Variables|Default|Get8))
  (bind _9 (Variables|Default|Get9))
  (bind _array (Utilities|Array|MakeArray _1 _2 _3 _4 _5 _6 _7 _8 _9 0))
  (Utilities|FlowControl|Delay (Variables|Default|GetActivationDelay) :!label _label)
  (Rendering|SetVisibility (Utilities|Array|Get(acopy) _array (Variables|Default|GetWallPieceIndex)) true false)
  (bind _result (Math|Integer|IncrementInt (Variables|Default|GetWallPieceIndex))
    (:%20%20
      (if (< _result (Utilities|Array|Length _array))
        (goto _label)
        (else
          (Variables|Default|SetWallPieceIndex 0))))))

(event EventHitCounter
  (params (Player :type MyTags%20Enum))
  (bind _playertag_set (Variables|Default|GetPlayerTag_set))
  (bind _5 (Variables|Default|Get5))
  (bind _1 (Variables|Default|Get1))
  (bind _2 (Variables|Default|Get2))
  (bind _3 (Variables|Default|Get3))
  (bind _4 (Variables|Default|Get4))
  (bind _6 (Variables|Default|Get6))
  (bind _7 (Variables|Default|Get7))
  (bind _8 (Variables|Default|Get8))
  (bind _9 (Variables|Default|Get9))
  (bind _array (Utilities|Array|MakeArray _1 _2 _3 _4 _5 _6 _7 _8 _9 0))
  (if (Utilities|Enum|Equal(Enum) _playertag_set Player)
    (Rendering|Material|SetMaterial (Utilities|Array|Get(acopy) _array (Variables|Default|GetWallPieceIndex)) 0 (Utilities|Select :Index _playertag_set :NewEnumerator0 "/Game/Materials/goal_red_off.goal_red_off" :NewEnumerator1 "/Game/Materials/goal_white_off.goal_white_off"))
    (bind _result (Math|Integer|IncrementInt (Variables|Default|GetWallPieceIndex))
      (:%20%20
        (if (< _result (Utilities|Array|Length _array))
          _)))))

(fn ConstructionScript)