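; HexWall_white is a player's wall of hex static mesh pieces that can be destroyed one at a time.
; DestroyHexPiece removes a given component and spawns a Tor_Treffer hit effect there, yawed toward the world origin.
; On Tick, the authority recounts remaining static mesh components and, when the total changes, writes it to the VR_GameMode wall count for Player 1 or 2 by PlayerTag.
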(event Custom|Destroy%20Hex%20Piece
  (params (Component :type Actor%20Component%20Object%20Reference) (Location :type Vector))
  (Components|DestroyComponent Component)
  (Effects|SpawnEmitteratLocation "/Game/ParticleEffects/Tor_Treffer.Tor_Treffer" Location (Math|Rotator|FindLookatRotation (* Location "1.000000,1.000000, 0") (Math|Vector|MakeVector 0.0 0.0 0.0))))

(event EventBeginPlay
  (bind _asvr_game_mode (Utilities|Casting|CastToVR_GameMode (Game|GetGameMode)))
  (Variables|Default|SetVR_GameMode _asvr_game_mode))

(event EventTick
  (params (DeltaSeconds :type Float%20%28single-precision%29))
  (bind _returnvalue (Actor|GetComponentsByClass "/Script/Engine.StaticMeshComponent"))
  (bind _vr_gamemode (Variables|Default|GetVR_GameMode))
  (bind _returnvalue_2 (Utilities|Array|Length _returnvalue))
  (Networking|SwitchHasAuthority
    (:Authority
      (if (!= (Variables|Default|GetWallPieces) _returnvalue_2)
        (Variables|Default|SetWallPieces _returnvalue_2)
        (switch Utilities|FlowControl|Switch|SwitchonMyTags (Variables|Default|GetPlayerTag)
          (:NewEnumerator0
            (Variables|/Game/Blueprints/VR_GameMode.VR_GameMode_C|SetHexWallCountP1 _vr_gamemode (Variables|Default|GetWallPieces)))
          (:NewEnumerator1
            (Variables|/Game/Blueprints/VR_GameMode.VR_GameMode_C|SetHexWallCountP2 _vr_gamemode (Variables|Default|GetWallPieces))))))))

(fn ConstructionScript)