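; Thrown VR disc projectile that flies, returns to its homing target (by default the player's right controller) and is destroyed on catch.
; The server switches on homing once horizontal velocity points back from the enemy direction, while clients interpolate toward the server-set transform.
; Hits spawn impact effects chosen by shield tag and enemy flag; the server breaks HexWall pieces and sends hit sound events to the game mode.
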(event OnComponentHit(Disc)
  (params (HitComponent :type Primitive%20Component%20Object%20Reference) (OtherActor :type Actor%20Object%20Reference) (OtherComp :type Primitive%20Component%20Object%20Reference) (NormalImpulse :type Vector :default "0, 0, 0") (Hit :type Hit%20Result%20Structure%20%28by%20ref%29))
  (Effects|SpawnEmitteratLocation (select (Components|ComponentHasTag OtherComp "Shield") "/Game/ParticleEffects/Shield_Collision.Shield_Collision" (select (Variables|Default|GetIsEnemy) 0 "/Game/ParticleEffects/Collision.Collision")) (.location Hit) (Math|Rotator|FindLookatRotation (.location Hit) (+ (.location Hit) (.normal Hit))))
  (Networking|SwitchHasAuthority
    (:Authority
      (CallFunction|HitHexWall OtherActor OtherComp (.location Hit)))))

(event Custom|Enable%20Homing
  (bind _projectilemovement (Variables|Default|GetProjectileMovement))
  (Variables|/Script/Engine.ProjectileMovementComponent|SetHomingTargetComponent _projectilemovement (Variables|Default|GetHomingTarget))
  (Variables|/Script/Engine.ProjectileMovementComponent|SetbIsHomingProjectile _projectilemovement true))

(event Custom|Enable%20Movement
  (params (Local%20Velocity :type Vector) (Is_Enemy :type Boolean))
  (bind _projectilemovement (Variables|Default|GetProjectileMovement))
  (Variables|Default|SetIsEnemy Is_Enemy)
  (Game|Components|ProjectileMovement|SetVelocityinLocalSpace _projectilemovement Local%20Velocity)
  (Physics|SetSimulatePhysics (Variables|Default|GetDisc) false)
  (Components|Activation|Activate _projectilemovement false)
  ;[0 0.9287 1] todo: Clientseitig; gegner braucht anderen Sound
  (Audio|SpawnSoundAttached "/Game/Sound/Disc_Throw_sfx.Disc_Throw_sfx" (Variables|Default|GetDisc_Flying_Cue))
  (Components|Activation|SetActive (Variables|Default|GetDisc_Flying_Cue) true false))

(event EventBeginPlay
  (bind _asvr_game_mode (Utilities|Casting|CastToVR_GameMode (Game|GetGameMode)))
  (Variables|Default|SetVR_GameMode _asvr_game_mode)
  (CallFunction|InitDisc))

(event EventTick
  (params (DeltaSeconds :type Float%20%28single-precision%29))
  (Networking|SwitchHasAuthority
    (:Authority
      (Variables|Default|SetActorTransformTarget (Transformation|GetActorTransform))
      (if (Components|Activation|IsActive (Variables|Default|GetProjectileMovement))
        (Utilities|IsValid (Variables|Default|GetHomingTarget)
          (:Is%20Valid
            (Utilities|FlowControl|Sequence
              (:then_0
                ;[1 1 1] Enable Homing when Disc is returning
                (if (> (Class|KismetMathLibrary|DegAcos (Math|Vector|DotProduct (Variables|Default|GetDirectionFromPlayerToEnemy) (Math|Vector|Normalize (* (Transformation|GetVelocity) "1.000000,1.000000, 0")))) 9e+01)
                  (Utilities|FlowControl|DoOnce true :!label _label
                    (:Completed
                      (CallFunction|EnableHoming)))
                  (else
                    (goto _label Reset))))
              (:then_1
                ;[1 1 1] Destroy Disc when returned
                (if (and (Variables|/Script/Engine.ProjectileMovementComponent|GetbIsHomingProjectile (Variables|Default|GetProjectileMovement)) (< (Math|Vector|VectorLength (- (Transformation|GetActorLocation) (Transformation|GetWorldLocation (Variables|Default|GetHomingTarget)))) 1e+02))
                  (Audio|SpawnSoundAttached "/Game/Sound/Disc_Catch_sfx_Cue.Disc_Catch_sfx_Cue" (Variables|Default|GetDisc))
                  (Actor|DestroyActor))))))))
    (:Remote
      (Transformation|SetActorTransform (Class|KismetMathLibrary|TInterpto (Transformation|GetActorTransform) (Variables|Default|GetActorTransformTarget) (Utilities|Time|GetWorldDeltaSeconds) 1e+01)))))

(fn ConstructionScript)

(fn HitHexWall
  (params (Other%20Actor :type Actor%20Object%20Reference) (Component :type Primitive%20Component%20Object%20Reference) (Location :type Vector))
  (bind _returnvalue (Game|GetGameMode))
  (bind _ashex_wall (Utilities|Casting|CastToHexWall Other%20Actor)
    (:then
      (Default|DestroyHexPiece _ashex_wall Component Location)
      ;[0 1 0.9206] //ToDo: Client Seitig bestgimmen Audiofeedback
      (Class|SoundManagerBPI|SoundHitEvent(Message) _returnvalue (Variables|Default|GetHit_Event_Name_Tag) Location))
    (:CastFailed
      (Utilities|Casting|CastToVR_Character Other%20Actor
        (:then
          (Class|SoundManagerBPI|SoundHitEvent(Message) _returnvalue "Hit_Shield" Location))
        (:CastFailed
          (Class|SoundManagerBPI|SoundHitEvent(Message) _returnvalue "Hit_Simple" Location)))))
  (return))

(fn InitDisc
  (Class|ActorComponent|SetIsReplicated (Variables|Default|GetProjectileMovement) true)
  (Utilities|IsValid (Variables|Default|GetHomingTarget)
    (:Is%20Valid
      (Variables|Default|SetDirectionFromPlayerToEnemy (Class|KismetMathLibrary|GetDirectionVector (* (Transformation|GetWorldLocation (Variables|Default|GetHomingTarget)) "0.000000,1.000000, 0") (Math|Vector|MakeVector 0.0 0.0 0.0)) :!label _label))
    (:Is%20Not%20Valid
      (bind _asvr_character (Utilities|Casting|CastToVR_Character (Game|Player|GetPlayerPawn 0))
        (:then
          (Variables|Default|SetHomingTarget (Variables|/Game/Blueprints/VR_Character.VR_Character_C|Getvr_controller_R _asvr_character))
          (goto _label))
        (:CastFailed
          _))))
  (return))