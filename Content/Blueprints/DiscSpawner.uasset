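; Disc spawner that keeps one enemy disc in play, launched from and homing on the spawner's root.
; A server-authority custom event checks whether its disc is still valid, then after a one-second delay spawns a replacement.
; The new disc gets the enemy mesh, a goal-against hit tag and flight audio, then movement along a local-space vector from a cone-direction function built around random spread and disc speed.
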(event Custom|CustomEvent
  (params (DeltaSeconds :type Float%20%28single-precision%29 :default 0.0))
  (Networking|SwitchHasAuthority
    (:Authority
      (Utilities|IsValid (Variables|Default|GetSpawnedDisc)
        (:Is%20Not%20Valid
          (Utilities|FlowControl|Delay 1.0)
          (bind _returnvalue (Game|SpawnActorfromClass "/Game/Blueprints/Disc.Disc_C" (Transformation|GetActorTransform) "Undefined" 0 0 (Variables|Default|GetDefaultSceneRoot)))
          (bind _output_get (Variables|Default|SetSpawnedDisc _returnvalue))
          (Class|SkinnedMeshComponent|SetSkeletalMesh (Variables|/Game/Blueprints/Disc.Disc_C|GetDisc _output_get) "/Game/Models/Disc_Enemy.Disc_Enemy" true)
          (Variables|/Game/Blueprints/Disc.Disc_C|SetHit_Event_Name_Tag (Variables|Default|GetSpawnedDisc) "Hit_GoalAgainst")
          (Effects|Components|ParticleSystem|SetIntParameter (Variables|/Game/Blueprints/Disc.Disc_C|GetFlyingDisc_Cue (Variables|Default|GetSpawnedDisc)) "Movement_Sound_Switch" 0)
          (Components|Activation|ToggleActive (Variables|/Game/Blueprints/Disc.Disc_C|GetFlyingDisc_Cue (Variables|Default|GetSpawnedDisc)))
          (Default|EnableMovement (Variables|Default|GetSpawnedDisc) (Math|Transform|InverseTransformDirection (Transformation|GetActorTransform (Variables|Default|GetSpawnedDisc)) (|GetDirectionInCone_2))))))))

(event EventBeginPlay)

(event Collision|EventActorBeginOverlap
  (params (OtherActor :type Actor%20Object%20Reference)))

(fn ConstructionScript)