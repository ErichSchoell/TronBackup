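; Game mode for a two-player VR match that tracks both players, teleporting the second to a MyPlayerStart on login.
; Once both are ready, it fires the game-ready event and counts down a timer copied to VR_GameState.
; Interface messages drive disc destruction, clock start and picture-widget hiding, and a named lookup plays hit sounds.
; Hex-wall win/draw logic with result text and level restart exists but is disconnected.
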(event Custom|Game_Ready_Event
  (bind _outactors (Actor|GetAllActorswithInterface "/Game/Blueprints/GameStart_BPI.GameStart_BPI_C"))
  (for _array_element _outactors
    (Class|GameStartBPI|StarttheClock(Message) _array_element)))

(event EventTick
  (params (DeltaSeconds :type Float%20%28single-precision%29))
  (bind _player_1 (Variables|Default|GetPlayer_1))
  (bind _player_2 (Variables|Default|GetPlayer_2))
  (Utilities|IsValid _player_1
    (:Is%20Valid
      (Utilities|IsValid _player_2
        (:Is%20Valid
          (if (and (Variables|/Game/Blueprints/VR_Character.VR_Character_C|GetPlayer_Ready _player_1) (Variables|/Game/Blueprints/VR_Character.VR_Character_C|GetPlayer_Ready _player_2))
            (Utilities|FlowControl|Sequence
              (:then_0
                (Utilities|FlowControl|DoOnce false
                  (:Completed
                    (CallFunction|GameReadyEvent))))
              (:then_1
                (CallFunction|UpdateTimer)))))))))

(event EventBeginPlay
  (CallFunction|InitGame))

(event EventKeyPressedSwitchPictures
  (params (KeyCode :type Integer))
  (switch int KeyCode
    (:0
      (bind _foundwidgets (Class|WidgetBlueprintLibrary|GetAllWidgetswithInterface "/Game/Blueprints/Picture_Switch_BPI.Picture_Switch_BPI_C" false))
      (for _array_element _foundwidgets
        (Class|PictureSwitchBPI|SwitchingPicturesNow(Message) _array_element false)))))

(event EventPostLogin
  (params (NewPlayer :type Player%20Controller%20Object%20Reference))
  (bind _returnvalue (Pawn|GetControlledPawn NewPlayer))
  (Utilities|FlowControl|Sequence
    (:then_0
      (bind _outactors (Actor|GetAllActorswithInterface "/Game/Blueprints/GameStart_BPI.GameStart_BPI_C"))
      (for _array_element _outactors
        (Class|GameStartBPI|DiscDestruction(Message) _array_element)))
    (:then_1
      (bind _returnvalue_2 (Class|GameMode|GetNumPlayers))
      (bind _asvr_character (Utilities|Casting|CastToVR_Character _returnvalue))
      (switch int _returnvalue_2
        (:2
          (bind _output_get (Variables|Default|SetPlayer_2 _asvr_character))
          (Variables|/Game/Blueprints/VR_Character.VR_Character_C|SetPlayerTag _output_get "NewEnumerator1")
          (bind _outactors_2 (Actor|GetAllActorsOfClass "/Game/Blueprints/MyPlayerStart.MyPlayerStart_C"))
          (Transformation|Teleport _returnvalue (.location (Transformation|GetActorTransform (Utilities|Array|Get(acopy) _outactors_2))) (.rotation (Transformation|GetActorTransform (Utilities|Array|Get(acopy) _outactors_2)))))))))

(event EventSoundHitEvent
  (params (Hit_Location :type String) (Hit_Sound_Location :type Vector))
  ;[1 1 1] Sound_Manager
  (Audio|PlaySoundatLocation (Utilities|Array|Get(acopy) (Variables|Default|GetEvent_Sounds) (Utilities|Array|FindItem (Variables|Default|GetEvent_Names) Hit_Location)) Hit_Sound_Location))

(fn ConstructionScript)

(fn InitGame
  (Variables|Default|SetTime (Variables|Default|GetMaxTime))
  (bind _asvr_character (Utilities|Casting|CastToVR_Character (Game|Player|GetPlayerPawn 0)))
  (Variables|Default|SetPlayer_1 _asvr_character))

(fn UpdateTimer
  (Variables|Default|SetTime (Math|Float|Clamp(Float) (- (Variables|Default|GetTime) (Utilities|Time|GetWorldDeltaSeconds)) 0.0 (Variables|Default|GetMaxTime)))
  (bind _asvr_game_state (Utilities|Casting|CastToVR_GameState (Game|GetGameState))
    (:then
      (Variables|/Game/Blueprints/VR_GameState.VR_GameState_C|SetTime _asvr_game_state (Variables|Default|GetTime)))
    (:CastFailed
      _))
  (return))

(fn SpawnText
  (params (Transform :type Transform) (Text :type Text) (Color :type Linear%20Color%20Structure))
  (bind _returnvalue (Game|SpawnActorfromClass "/Script/Engine.TextRenderActor" Transform "Undefined" 0 0))
  (Rendering|Components|TextRender|SetText (Variables|/Script/Engine.TextRenderActor|GetTextRender _returnvalue) (Utilities|Text|MakeLiteralText Text))
  (Rendering|Components|TextRender|SetHorizontalAlignment (Variables|/Script/Engine.TextRenderActor|GetTextRender _returnvalue) "EHTA_Center")
  (Rendering|Components|TextRender|SetWorldSize (Variables|/Script/Engine.TextRenderActor|GetTextRender _returnvalue) 1e+02)
  (Rendering|Components|TextRender|SetTextRenderColor (Variables|/Script/Engine.TextRenderActor|GetTextRender _returnvalue) (Math|Conversions|ToColor(LinearColor) Color))
  (return))