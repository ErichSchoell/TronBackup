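; Game start countdown clock that lights three white and red element pairs in turn, then releases the start.
; Construction script fills arrays of lights and sound points, which StarttheClock steps through each second, swapping materials and playing a get-ready cue.
; After the third step it sends hex-wall toggle and disc destruction messages to all GameStart_BPI actors.
; Following a short delay, it switches all lights to basic glow and plays the go sound.
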(event EventStarttheClock
  (Rendering|Material|SetMaterial (Utilities|Array|Get(acopy) (Variables|Default|GetClock_Ref_List_White) (Variables|Default|GetCopuntDown_Ref)) 0 "/Game/Materials/goal_white.goal_white" :!label _label)
  (Rendering|Material|SetMaterial (Utilities|Array|Get(acopy) (Variables|Default|GetClock_Ref_List_Red) (Variables|Default|GetCopuntDown_Ref)) 0 "/Game/Materials/goal_red.goal_red")
  (Audio|PlaySoundatLocation "/Game/Sound/Get_Ready_sfx_Cue.Get_Ready_sfx_Cue" (Transformation|GetWorldLocation (Utilities|Array|Get(acopy) (Variables|Default|GetSound_Ref_List) (Variables|Default|GetCopuntDown_Ref))))
  (Utilities|FlowControl|Delay 1.0)
  (Variables|Default|SetCopuntDown_Ref (+ (Variables|Default|GetCopuntDown_Ref) 1))
  (if (== (Variables|Default|GetCopuntDown_Ref) 3)
    (bind _outactors (Actor|GetAllActorswithInterface "/Game/Blueprints/GameStart_BPI.GameStart_BPI_C"))
    (for _array_element _outactors
      (Class|GameStartBPI|HexWallToggleCall(Message) _array_element)
      (Class|GameStartBPI|DiscDestruction(Message) _array_element))
    (Utilities|FlowControl|Delay 2.1)
    (for _array_element_2 (Variables|Default|GetClock_Ref_List_White)
      (Rendering|Material|SetMaterial _array_element_2 0 "/Game/Materials/basic_glow_white.basic_glow_white"))
    (for _array_element_3 (Variables|Default|GetClock_Ref_List_Red)
      (Rendering|Material|SetMaterial _array_element_3 0 "/Game/Materials/basic_glow_red.basic_glow_red"))
    (bind _returnvalue (Audio|SpawnSoundatLocation "/Game/Sound/Go_sfx_Cue.Go_sfx_Cue" (Transformation|GetWorldLocation (Variables|Default|GetDefaultSceneRoot))))
    ;[1 1 1] Sound Debug
    (Effects|Components|ParticleSystem|SetIntParameter _returnvalue "Sound_Switch" 0)
    (Utilities|FlowControl|Delay 0.2)
    (else
      (goto _label))))

(fn ConstructionScript
  (bind _clock_ref_list_white (Variables|Default|GetClock_Ref_List_White))
  (bind _sound_ref_list (Variables|Default|GetSound_Ref_List))
  (bind _clock_ref_list_red (Variables|Default|GetClock_Ref_List_Red))
  (Utilities|FlowControl|Sequence
    (:then_0
      (Utilities|Array|Add _clock_ref_list_white (Variables|Default|GetWhite_1))
      (Utilities|Array|Add _clock_ref_list_white (Variables|Default|GetWhite_2))
      (Utilities|Array|Add _clock_ref_list_white (Variables|Default|GetWhite_3)))
    (:then_1
      (Utilities|Array|Add _clock_ref_list_red (Variables|Default|GetRed_1))
      (Utilities|Array|Add _clock_ref_list_red (Variables|Default|GetRed_2))
      (Utilities|Array|Add _clock_ref_list_red (Variables|Default|GetRed_3)))
    (:then_2
      (Utilities|Array|Add _sound_ref_list (Variables|Default|GetSound_1))
      (Utilities|Array|Add _sound_ref_list (Variables|Default|GetSound_2))
      (Utilities|Array|Add _sound_ref_list (Variables|Default|GetSound_3)))))