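; An optional banner actor whose picture can be swapped or hidden on demand.
; SwitchingPicturesNow forwards a visibility flag and an image to a switch event, which branches to Switch or Off.
; Switch shows the BannerOptional component and applies the image as the material in its first slot, while Off hides the component.
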(event Custom|Switch_Event
  (params (Visible :type Boolean) (Image :type Material%20Instance%20Object%20Reference))
  (if Visible
    (CallFunction|Switch Image)
    (else
      (CallFunction|Off))))

(event EventBeginPlay)

(event Collision|EventActorBeginOverlap
  (params (OtherActor :type Actor%20Object%20Reference)))

(event EventSwitchingPicturesNow
  (params (Visible :type Boolean) (Image :type Material%20Instance%20Object%20Reference))
  (CallFunction|SwitchEvent Visible Image))

(event EventTick
  (params (DeltaSeconds :type Float%20%28single-precision%29)))

(fn ConstructionScript)

(fn Switch
  (params (Image :type Material%20Instance%20Object%20Reference))
  (bind _banner_optional (Variables|Default|Getbanner_optional))
  (Rendering|SetVisibility _banner_optional true false)
  (Rendering|Material|SetMaterial _banner_optional 0 Image))

(fn Off
  (Rendering|SetVisibility (Variables|Default|Getbanner_optional) false false))